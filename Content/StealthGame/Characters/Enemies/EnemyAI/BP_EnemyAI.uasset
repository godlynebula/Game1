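; Stealth-game enemy AI that patrols, investigates noises, chases the player and melee-attacks, sending a caught player back to a checkpoint.
; Tick picks chase, looped target-point patrol or random roaming, using CanMove to gate new patrol moves.
; PawnSensing drives sight, which lapses via a retriggerable delay, and sends the AI toward noises.
; A montage notify fires a hand-socket sphere trace; a DoOnce re-arms attacks only while Hostile, which a hit clears.
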(event OnSeePawn(PawnSensing)
  (params (Pawn :type Pawn%20Object%20Reference))
  ;[0.15 0.15 0.15 0.5] Sets Booleans to Tell AI if it can see the Player
  (Utilities|FlowControl|Sequence
    (:then_0
      (Utilities|Casting|CastToBP_ThirdPersonCharacterCustom Pawn
        (:then
          (Development|PrintString "Hey, stop right there!")
          (Variables|Default|SetbPlayerVisible true)
          (Development|SetHiddeninGame (Variables|Default|GetCube) false false)
          (Utilities|FlowControl|Delay 2.0)
          (Development|SetHiddeninGame (Variables|Default|GetCube) true false))
        (:CastFailed
          (Variables|Default|SetbPlayerVisible false))))
    (:then_1
      (Utilities|FlowControl|RetriggerableDelay 1.0)
      (Development|PrintString "Must've been the wind...")
      (Variables|Default|SetbPlayerVisible false))))

(event OnHearNoise(PawnSensing)
  (params (Instigator :type Pawn%20Object%20Reference) (Location :type Vector%20%28by%20ref%29 :default "0, 0, 0") (Volume :type Float%20%28single-precision%29))
  ;[0.15 0.15 0.15 0.5] Gives AI Ability to Hear Objects
  (CallFunction|UpdateWalkSpeed 2e+02)
  (Variables|Default|SetbCanMove false)
  (AI|AIMoveTo self Location Instigator 5e+01 false
    (:OnSuccess
      _)
    (:OnFail
      _))
  (Utilities|FlowControl|Delay 6.0) ; Rock Distraction Time
  (Variables|Default|SetbCanMove true))

(event Custom|ChasePlayer
  ;[0.15 0.15 0.15 0.5] Tells the AI to Chase Player and Attack the Player
  (CallFunction|UpdateWalkSpeed 6e+02)
  (Variables|Default|SetbCanMove false)
  (AI|AIMoveTo self "0, 0, 0" (Game|GetPlayerCharacter 0) 5e+01 false
    (:OnSuccess
      (CallFunction|Attack)
      (Utilities|FlowControl|Delay 3.0)
      (Variables|Default|SetbCanMove true))))

(event Custom|PatrolRandom
  ;[0.15 0.15 0.15 0.5] Tells the AI to Patrol Randomly in a Specific Radius
  (CallFunction|UpdateWalkSpeed 2e+02)
  (Variables|Default|SetbCanMove false)
  (AI|AIMoveTo self (.RandomLocation (AI|Navigation|GetRandomReachablePointinRadius (Transformation|GetActorLocation) 2e+03 0 0)) 0 5e+01 false
    (:OnSuccess
      _)
    (:OnFail
      _))
  (Utilities|FlowControl|Delay 3.0)
  (Variables|Default|SetbCanMove true))

(event Custom|SetNextPatrolPointIndex
  ;[0.15 0.15 0.15 0.5] Sets Next Patrol Point in the Index for AI to Move Towards
  (Variables|Default|SetPatrolTargetPointIndex (Math|Integer|%(Integer) (+ (Variables|Default|GetPatrolTargetPointIndex) 1) (Utilities|Array|Length (Variables|Default|GetPatrolTargetPoints)))))

(event Custom|MoveToNextPatrolPoint
  ;[0.15 0.15 0.15 0.5] Tells the AI to Move to the Next Patrol Point
  (CallFunction|UpdateWalkSpeed 2e+02)
  (Variables|Default|SetbCanMove false)
  (AI|AIMoveTo self "0, 0, 0" (Utilities|Array|Get(acopy) (Variables|Default|GetPatrolTargetPoints) (Variables|Default|GetPatrolTargetPointIndex)) 5e+01 false
    (:OnSuccess
      (Utilities|FlowControl|Delay 3.0)
      (Variables|Default|SetbCanMove true)
      (CallFunction|SetNextPatrolPointIndex))))

(event Custom|Attack
  (bind _mesh (Variables|Character|GetMesh))
  (bind _returnvalue (Transformation|GetSocketLocation _mesh "hand_r"))
  ;[0.15 0.1407 0.04319 0.5] Bonk (The Attack Blueprint)
  (Utilities|FlowControl|DoOnce false ; Only Reset Attack on miss.
    (:Completed
      (bind _notifyname (Animation|Montage|PlayMontage (Variables|Character|GetMesh) "/Game/StealthGame/Characters/Enemies/AM_Attack_01.AM_Attack_01") ; Play the AM_Attack_01
        (:OnCompleted
          (if (Variables|Default|GetbHostile)
            (CallFunction|ResetAttack) ; Resets the Do Once node.
          ))
        (:OnNotifyBegin
          (switch name _notifyname ; Pick the proper attack type(standard when there is more than one type of attack)
            (:AttackDamage
              (Development|PrintString "I'm attacking!")
              (bind (_outhits _returnvalue_2) (Collision|MultiSphereTraceForObjects _returnvalue (+ _returnvalue (* (Transformation|GetActorForwardVector) (Variables|Default|GetMeleeTraceDistance))) (Variables|Default|GetMeleeTraceRadius) (Utilities|Array|MakeArray "ObjectTypeQuery3") false 0 "None")) ; Trace forward from hand socket.
              (if _returnvalue_2 ; If a pawn is hit in that trace...
                (for _array_element _outhits ; ...loop through the results....
                  (bind _asbp_third_person_character_custom (Utilities|Casting|CastToBP_ThirdPersonCharacterCustom (.HitActor (Collision|BreakHitResult _array_element))))
                  (Default|LoadCheckpoint _asbp_third_person_character_custom)
                  (Variables|Default|SetbHostile false))))))))))

(event Custom|ResetAttack
  (bind _mesh (Variables|Character|GetMesh))
  (bind _returnvalue (Transformation|GetSocketLocation _mesh "hand_r"))
  ;[0.15 0.1407 0.04319 0.5] Bonk (The Attack Blueprint)
  (Utilities|FlowControl|DoOnce false) ; enters at Reset
)

(event EventTick
  (params (DeltaSeconds :type Float%20%28single-precision%29))
  ;[0.15 0.15 0.15 0.5] Series of Branch Nodes that Checks Bools Every Tick to Determine the AI's Plan of Action
  (if (Variables|Default|GetbCanMove)
    (if (Variables|Default|GetbPlayerVisible)
      (CallFunction|ChasePlayer)
      (elif (Variables|Default|GetbTargetPointMovement)
        (CallFunction|MovetoNextPatrolPoint)
        (else
          (CallFunction|PatrolRandom))))
    (elif (Variables|Default|GetbPlayerVisible)
      (CallFunction|ChasePlayer))))

(fn ConstructionScript)

(fn UpdateWalkSpeed
  (params (NewWalkSpeed :type Float%20%28double-precision%29))
  (Variables|/Script/Engine.CharacterMovementComponent|SetMaxWalkSpeed (Variables|Character|GetCharacterMovement) NewWalkSpeed))
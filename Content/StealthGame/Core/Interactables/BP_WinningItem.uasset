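; BP_WinningItem is a collectible that the player character picks up by touching it, which opens a reward choice screen.
; On sphere overlap it increments the character's WinningItemCount, sets HasWinningItem and fires the OnWinningItemCollected dispatcher.
; It destroys itself, then in the same execution chain shows W_RewardChoice, switches to UI-only input with a visible cursor and disables character input.
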(event OnComponentBeginOverlap(Sphere)
  (params (OverlappedComponent :type Primitive%20Component%20Object%20Reference) (OtherActor :type Actor%20Object%20Reference) (OtherComp :type Primitive%20Component%20Object%20Reference) (OtherBodyIndex :type Integer) (bFromSweep :type Boolean) (SweepResult :type Hit%20Result%20Structure%20%28by%20ref%29))
  (bind _returnvalue (Game|GetPlayerController 0))
  (bind _asbp_third_person_character_custom (Utilities|Casting|CastToBP_ThirdPersonCharacterCustom OtherActor))
  (Development|PrintString "Winning Item Overlapped by Player!" true true "(R=0.000000,G=0.660000,B=1.000000,A=1.000000)" 5.0)
  (Variables|/Game/StealthGame/Core/Characters/PlayerCharacter/BP_ThirdPersonCharacterCustom.BP_ThirdPersonCharacterCustom_C|SetWinningItemCount _asbp_third_person_character_custom (+ (Variables|/Game/StealthGame/Core/Characters/PlayerCharacter/BP_ThirdPersonCharacterCustom.BP_ThirdPersonCharacterCustom_C|GetWinningItemCount _asbp_third_person_character_custom) 1))
  (Variables|/Game/StealthGame/Core/Characters/PlayerCharacter/BP_ThirdPersonCharacterCustom.BP_ThirdPersonCharacterCustom_C|SetbHasWinningItem _asbp_third_person_character_custom true)
  (Default|CallOnWinningItemCollected)
  (Actor|DestroyActor) ; Destroy this key
  (bind _returnvalue_2 (UserInterface|CreateWidget "/Game/StealthGame/MaterialLibrary/Widgets/W_RewardChoice.W_RewardChoice_C"))
  (bind _output_get (Variables|Default|SetRewardWidget _returnvalue_2))
  (UserInterface|Viewport|AddtoViewport _output_get 0)
  (Input|SetInputModeUIOnly _returnvalue (Variables|Default|GetRewardWidget) "DoNotLock" false)
  (Variables|/Script/Engine.PlayerController|SetbShowMouseCursor _returnvalue true)
  (Input|DisableInput (Game|GetPlayerCharacter 0) _returnvalue))

(event EventBeginPlay)

(event Collision|EventActorBeginOverlap
  (params (OtherActor :type Actor%20Object%20Reference)))

(event EventTick
  (params (DeltaSeconds :type Float%20%28single-precision%29)))

(fn ConstructionScript)
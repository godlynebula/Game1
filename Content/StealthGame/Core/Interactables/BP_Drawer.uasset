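; BP_Drawer is an interactable drawer in the stealth game that holds a key for the player to collect.
; Its interaction box overlaps set the player character's CanInteract flag and register the drawer as CurrentDrawer, which is not cleared on exit.
; InteractWithDrawer steps through three states: a timeline slides the drawer open, the key count increments as two cylinder meshes hide, then it prints that it is empty.
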(event OnComponentBeginOverlap(InteractionBox)
  (params (OverlappedComponent :type Primitive%20Component%20Object%20Reference) (OtherActor :type Actor%20Object%20Reference) (OtherComp :type Primitive%20Component%20Object%20Reference) (OtherBodyIndex :type Integer) (bFromSweep :type Boolean) (SweepResult :type Hit%20Result%20Structure%20%28by%20ref%29))
  (bind _asbp_third_person_character_custom (Utilities|Casting|CastToBP_ThirdPersonCharacterCustom OtherActor))
  (Variables|/Game/StealthGame/Core/Characters/PlayerCharacter/BP_ThirdPersonCharacterCustom.BP_ThirdPersonCharacterCustom_C|SetbCanInteract _asbp_third_person_character_custom true)
  (Variables|Default|SetbNearDrawer true)
  (Variables|/Game/StealthGame/Core/Characters/PlayerCharacter/BP_ThirdPersonCharacterCustom.BP_ThirdPersonCharacterCustom_C|SetCurrentDrawer _asbp_third_person_character_custom self))

(event OnComponentEndOverlap(InteractionBox)
  (params (OverlappedComponent :type Primitive%20Component%20Object%20Reference) (OtherActor :type Actor%20Object%20Reference) (OtherComp :type Primitive%20Component%20Object%20Reference) (OtherBodyIndex :type Integer))
  (bind _asbp_third_person_character_custom (Utilities|Casting|CastToBP_ThirdPersonCharacterCustom OtherActor))
  (Variables|/Game/StealthGame/Core/Characters/PlayerCharacter/BP_ThirdPersonCharacterCustom.BP_ThirdPersonCharacterCustom_C|SetbCanInteract _asbp_third_person_character_custom false)
  (Variables|Default|SetbNearDrawer false)
  (Variables|/Game/StealthGame/Core/Characters/PlayerCharacter/BP_ThirdPersonCharacterCustom.BP_ThirdPersonCharacterCustom_C|SetCurrentDrawer _asbp_third_person_character_custom self))

(event Custom|InteractWithDrawer
  (switch int (Variables|Default|GetDrawerCurrentState)
    (:0
      (Variables|Default|SetDrawerCurrentState 1)
      (bind _newtrack_0 (Timeline|Open%20Drawer Play)
        (:Update
          (Transformation|SetRelativeLocation (Variables|Default|GetBDrawer) (Math|Vector|Lerp(Vector) "0.000000,10.614418,-13.747886" "0.000000,90.614418,-13.747886" _newtrack_0) false false))))
    (:1
      (Variables|Default|SetDrawerCurrentState 2)
      (bind _asbp_third_person_character_custom (Utilities|Casting|CastToBP_ThirdPersonCharacterCustom (Game|GetPlayerCharacter 0)))
      (Development|PrintString "Player is Claiming a Key!" true true "(R=0.000000,G=0.660000,B=1.000000,A=1.000000)" 5.0)
      (Variables|/Game/StealthGame/Core/Characters/PlayerCharacter/BP_ThirdPersonCharacterCustom.BP_ThirdPersonCharacterCustom_C|SetKey%20Count _asbp_third_person_character_custom (+ (Variables|/Game/StealthGame/Core/Characters/PlayerCharacter/BP_ThirdPersonCharacterCustom.BP_ThirdPersonCharacterCustom_C|GetKey%20Count _asbp_third_person_character_custom) 1)) ; Set Key Count
      (Development|SetHiddeninGame (Variables|Default|GetCylinder) true false)
      (Development|SetHiddeninGame (Variables|Default|GetCylinder1) true false))
    (:2
      (Development|PrintString "drawer is empty"))))

(event EventBeginPlay
  (Variables|Default|SetDrawerCurrentState 0))

(fn ConstructionScript)
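; BP_FenceDoor is a one-sided fence door that the player character can only unblock from one side.
; An overlap trigger on the blocked side prints a message while the door is closed.
; The UnblockDoor trigger sets IsDoorOpen once, then the MoveWood timeline swings the board pivot.
; A 1.5-second delay, chained from that timeline's Update, starts the OpenDoor timeline that rotates the door pivot open.
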(event OnComponentBeginOverlap(IsDoorOpen?)
  (params (OverlappedComponent :type Primitive%20Component%20Object%20Reference) (OtherActor :type Actor%20Object%20Reference) (OtherComp :type Primitive%20Component%20Object%20Reference) (OtherBodyIndex :type Integer) (bFromSweep :type Boolean) (SweepResult :type Hit%20Result%20Structure%20%28by%20ref%29))
  (Utilities|Casting|CastToBP_ThirdPersonCharacterCustom OtherActor)
  (if (not (Variables|Default|GetbIsDoorOpen))
    (Development|PrintString "This door is blocked from the other side...")))

(event OnComponentBeginOverlap(UnblockDoor)
  (params (OverlappedComponent :type Primitive%20Component%20Object%20Reference) (OtherActor :type Actor%20Object%20Reference) (OtherComp :type Primitive%20Component%20Object%20Reference) (OtherBodyIndex :type Integer) (bFromSweep :type Boolean) (SweepResult :type Hit%20Result%20Structure%20%28by%20ref%29))
  (Utilities|Casting|CastToBP_ThirdPersonCharacterCustom OtherActor)
  (if (not (Variables|Default|GetbIsDoorOpen))
    (Variables|Default|SetbIsDoorOpen true)
    (bind _newtrack_0 (Timeline|Move%20Wood Play)
      (:Update
        (Development|PrintText "unblocking")
        (Transformation|SetRelativeRotation (Variables|Default|GetBoardPivot) (Math|Rotator|Lerp(Rotator) "0, 0, 0" "-90.000000,0.000000,0.000000" _newtrack_0) false false)
        (Utilities|FlowControl|Delay 1.5)
        (bind _newtrack_0_2 (Timeline|Open%20Door Play)
          (:Update
            (Transformation|SetRelativeRotation (Variables|Default|GetDoorPivot) (Math|Rotator|Lerp(Rotator) "0, 0, 0" "0.000000,-90.000000,0.000000" _newtrack_0_2) false false)))))))

(event EventBeginPlay)

(event Collision|EventActorBeginOverlap
  (params (OtherActor :type Actor%20Object%20Reference)))

(event EventTick
  (params (DeltaSeconds :type Float%20%28single-precision%29)))

(fn ConstructionScript)